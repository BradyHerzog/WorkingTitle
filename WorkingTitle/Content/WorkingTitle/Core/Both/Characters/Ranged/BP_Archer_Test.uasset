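; Test ranged archer actor that periodically fires BP_Arrow projectiles at the BP_FPChar_Sharpshooter character.
; A looping timer started on BeginPlay finds the target and solves the projectile-arc equation from horizontal distance, height difference, Velocity and Gravity.
; When the discriminant is non-negative, it spawns an arrow at its own location, pitched to the lower of the two launch angles and yawed toward the target.
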(event `self.ReceiveBeginPlay`
  (`KismetSystemLibrary.K2_SetTimerDelegate` (delegate `CustomEvent_0`) 2.0 true))

(event `CustomEvent_0`
  (bind _returnvalue (`self.K2_GetActorLocation`))
  (bind (_returnvalue_x _returnvalue_y _returnvalue_z) (`KismetMathLibrary.BreakVector` (`self.K2_GetActorLocation`)))
  (bind _gravity (`self.Gravity`))
  (bind _returnvalue_2 (`KismetMathLibrary.Square` (`self.Velocity`)))
  (bind _returnvalue_3 (`GameplayStatics.GetActorOfClass` "/Game/WorkingTitle/Core/FirstPerson/Characters/BP_FPChar_Sharpshooter.BP_FPChar_Sharpshooter_C"))
  (bind (_returnvalue_x_2 _returnvalue_y_2 _returnvalue_z_2) (`KismetMathLibrary.BreakVector` (`self.K2_GetActorLocation` _returnvalue_3)))
  (bind _returnvalue_4 (`KismetMathLibrary.VSize2D` (`KismetMathLibrary.MakeVector2D` (- _returnvalue_x_2 _returnvalue_x) (- _returnvalue_y_2 _returnvalue_y))))
  (bind _returnvalue_5 (- (`KismetMathLibrary.Square` _returnvalue_2) (* (+ (* (`KismetMathLibrary.Square` _returnvalue_4) _gravity) (* (* (- _returnvalue_z_2 _returnvalue_z) _returnvalue_2) 2.0)) _gravity)))
  (if (>= _returnvalue_5 0.0)
    (bind (_returnvalue_roll _returnvalue_pitch _returnvalue_yaw) (`KismetMathLibrary.BreakRotator` (`KismetMathLibrary.FindLookAtRotation` _returnvalue (`self.K2_GetActorLocation` _returnvalue_3))))
    (bind _returnvalue_6 (`KismetMathLibrary.Sqrt` _returnvalue_5))
    (bind _returnvalue_7 (* _returnvalue_4 _gravity))
    (`|SpawnActorFromClass` "/Game/WorkingTitle/Core/Both/Characters/BasicMelee/BP_Arrow.BP_Arrow_C" (`KismetMathLibrary.MakeTransform` _returnvalue (`KismetMathLibrary.MakeRotator` _returnvalue_roll (`KismetMathLibrary.FMin` (`KismetMathLibrary.DegAtan` (/ (+ _returnvalue_6 _returnvalue_2) _returnvalue_7)) (`KismetMathLibrary.DegAtan` (/ (- _returnvalue_2 _returnvalue_6) _returnvalue_7))) _returnvalue_yaw)) "Undefined" "OverrideRootScale" null null)))

(fn `UserConstructionScript`)