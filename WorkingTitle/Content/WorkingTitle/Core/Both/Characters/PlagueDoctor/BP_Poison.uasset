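; BP_Poison is a Plague Doctor poison actor that deals damage over time to the character that owns it.
; A one-second timer starts on BeginPlay, and each tick passes the owner, cast to BP_FPChar_Base, to ServerDamage, which calls TakeDamage with DamageToInflict.
; The timer re-arms after each hit until the TimeDamaged counter reaches TimesToDamage, when the actor destroys itself.
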(event `self.ReceiveBeginPlay`
  (`self.SetTimer`))

(event `SetTimer`
  (`KismetSystemLibrary.K2_SetTimerDelegate` (delegate `PoisionDamage`) 1.0))

(event `PoisionDamage`
  (`self.ServerDamage` (cast `/Game/WorkingTitle/Core/FirstPerson/Characters/BP_FPChar_Base` (`self.GetOwner`) :!pure true))
  (bind _result (`/Engine/EditorBlueprintResources/StandardMacros.IncrementInt` (`self.TimeDamaged`))
    (:`  `
      (if (== _result (`self.TimesToDamage`))
        (`self.K2_DestroyActor`)
        (else
          (`self.SetTimer`))))))

(event `ServerDamage`
  (params (DamageTarget :type "/Game/WorkingTitle/Core/FirstPerson/Characters/BP_FPChar_Base Object Reference"))
  (`/Game/WorkingTitle/Core/FirstPerson/Characters/BP_FPChar_Base.TakeDamage` DamageTarget (`self.DamageToInflict`)))

(fn `UserConstructionScript`)