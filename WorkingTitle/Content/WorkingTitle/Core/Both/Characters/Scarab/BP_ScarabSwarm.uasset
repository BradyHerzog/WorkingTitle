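; BP_ScarabSwarm is a wandering scarab swarm hazard that damages player characters standing in it.
; It loops AI moves to random nearby navigable points, retrying until one lies within a forward-facing world yaw window or too many retries fail, then turns toward it.
; Box overlaps track BP_FPChar_Base characters in an array, which a self-repeating delayed event damages slightly every second.
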(event `self.ReceiveBeginPlay`
  (`self.Move`)
  (`self.DamageRepeat`))

(event `Move`
  (bind _randomlocation (`NavigationSystemV1.K2_GetRandomLocationInNavigableRadius` (`self.K2_GetActorLocation`) 100.0 null null))
  (if (<= (`self.FailedPoints`) 25)
    (bind (_returnvalue_roll _returnvalue_pitch _returnvalue_yaw) (`KismetMathLibrary.BreakRotator` (`KismetMathLibrary.FindLookAtRotation` (`self.K2_GetActorLocation`) _randomlocation)))
    (if (`KismetMathLibrary.InRange_FloatFloat` _returnvalue_yaw -45.0 45.0)
      (set `self.FailedPoints` 0 :!label _label)
      (`self.K2_SetActorRotation` (`KismetMathLibrary.MakeRotator` 0.0 0.0 _returnvalue_yaw))
      (`|AIMoveTo` self _randomlocation null
        (:`OnSuccess`
          _)
        (:`OnFail`
          _))
      (`self.Move`)
      (else
        (`self.Move`)
        (`/Engine/EditorBlueprintResources/StandardMacros.IncrementInt` (`self.FailedPoints`))))
    (else
      (goto _label))))

(event `self.BoxCollision.OnComponentBeginOverlap`
  (params (OverlappedComponent :type "PrimitiveComponent Object Reference") (OtherActor :type "Actor Object Reference") (OtherComp :type "PrimitiveComponent Object Reference") (OtherBodyIndex :type Integer) (bFromSweep :type Boolean) (SweepResult :type "HitResult Structure (by ref)"))
  (bind _asbp_fpchar_base (cast `/Game/WorkingTitle/Core/FirstPerson/Characters/BP_FPChar_Base` OtherActor))
  (`KismetArrayLibrary.Array_Add` (`self.PlayersToDamage`) _asbp_fpchar_base))

(event `self.BoxCollision.OnComponentEndOverlap`
  (params (OverlappedComponent :type "PrimitiveComponent Object Reference") (OtherActor :type "Actor Object Reference") (OtherComp :type "PrimitiveComponent Object Reference") (OtherBodyIndex :type Integer))
  (bind _asbp_fpchar_base (cast `/Game/WorkingTitle/Core/FirstPerson/Characters/BP_FPChar_Base` OtherActor))
  (`KismetArrayLibrary.Array_RemoveItem` (`self.PlayersToDamage`) _asbp_fpchar_base))

(event `DamageRepeat`
  (for _array_element (`self.PlayersToDamage`)
    (`/Game/WorkingTitle/Core/FirstPerson/Characters/BP_FPChar_Base.TakeDamage` _array_element 0.5))
  (`KismetSystemLibrary.Delay` 1.0)
  (`self.DamageRepeat`))

(fn `UserConstructionScript`)