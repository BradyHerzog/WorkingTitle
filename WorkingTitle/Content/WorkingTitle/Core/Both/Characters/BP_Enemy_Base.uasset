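; Base enemy character with health, a floating health bar and death into a corpse.
; Damage requests route through ApplyDamage into AnyDamage, which lowers Health; its RepNotify calls Die at zero or below.
; Die traces downward to spawn a corpse at the hit location, then destroys the enemy.
; Each tick, the health bar shows only near the local player's screen center and yaws toward that player.
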(event `self.ReceiveBeginPlay`
  (set `self.Health` (`self.MaxHealth`))
  (bind _aswbp_enemy_health_bar (cast `/Game/WorkingTitle/Core/Both/Characters/BasicMelee/WBP_Enemy_HealthBar` (`WidgetComponent.GetUserWidgetObject` (`self.HealthBar`))))
  (set `/Game/WorkingTitle/Core/Both/Characters/BasicMelee/WBP_Enemy_HealthBar.OwningEnemy` self _aswbp_enemy_health_bar))

(event `Die`
  (bind _returnvalue (`SceneComponent.K2_GetComponentLocation` (`self.CapsuleComponent`)))
  (bind _outhit (`KismetSystemLibrary.LineTraceSingleForObjects` :`Start` _returnvalue :`End` (+ _returnvalue (0.0 0.0 -100000.0)) :`ObjectTypes` (`|MakeArray` "ObjectTypeQuery9" :!type "EObjectTypeQuery Enum") :`DrawDebugType` "Persistent"))
  (`|SpawnActorFromClass` "/Game/WorkingTitle/Core/Both/Characters/BP_Enemy_Corpse.BP_Enemy_Corpse_C" (`KismetMathLibrary.Conv_VectorToTransform` (`.Location` (`GameplayStatics.BreakHitResult` _outhit))) "AlwaysSpawn" "OverrideRootScale" null null)
  (`self.K2_DestroyActor`))

(event `self.ReceiveTick`
  (params (DeltaSeconds :type "Float (single-precision)"))
  (`self.RotateHealthBar`))

(event `RotateHealthBar`
  (bind _returnvalue (`GameplayStatics.GetPlayerController` 0))
  (bind (_sizex _sizey) (`PlayerController.GetViewportSize` _returnvalue))
  (bind _returnvalue_2 (<= (`KismetMathLibrary.VSize2D` (- (`KismetMathLibrary.MakeVector2D` (`KismetMathLibrary.Conv_IntToDouble` (/ _sizex 2)) (`KismetMathLibrary.Conv_IntToDouble` (/ _sizey 2))) (`PlayerController.ProjectWorldLocationToScreen` _returnvalue (`SceneComponent.K2_GetComponentLocation` (`self.HealthBar`)) true))) 150.0))
  (`/Engine/EditorBlueprintResources/StandardMacros.IsValid` _returnvalue
    (:`Is Valid`
      (`SceneComponent.SetVisibility` (`self.HealthBar`) _returnvalue_2 false)
      (if _returnvalue_2
        (bind _asbp_fpchar_base (cast `/Game/WorkingTitle/Core/FirstPerson/Characters/BP_FPChar_Base` (`Controller.K2_GetPawn` (`GameplayStatics.GetPlayerController` 0))))
        (bind (_returnvalue_roll _returnvalue_pitch _returnvalue_yaw) (`KismetMathLibrary.BreakRotator` (`KismetMathLibrary.FindLookAtRotation` (`self.K2_GetActorLocation`) (`self.K2_GetActorLocation` _asbp_fpchar_base))))
        (`SceneComponent.K2_SetWorldRotation` (`self.HealthBar`) (`KismetMathLibrary.MakeRotator` 0.0 0.0 _returnvalue_yaw) false false)))))

(event `Damage`
  (params (DamageAmmount :type "Float (double-precision)") (DamageCauser :type "Actor Object Reference"))
  ;[0 0 0] Damage
  (`GameplayStatics.ApplyDamage` self DamageAmmount (`self.GetInstigatorController` DamageCauser) DamageCauser "/Script/Engine.DamageType"))

(event `self.ReceiveAnyDamage`
  (params (Damage :type "Float (single-precision)") (DamageType :type "DamageType Object Reference") (InstigatedBy :type "Controller Object Reference") (DamageCauser :type "Actor Object Reference"))
  ;[0 0 0] Damage
  (set `self.Health` (- (`self.Health`) Damage)))

(fn `OnRep_Health`
  (if (<= (`self.Health`) 0.0)
    (`self.Die`)))

(fn `UserConstructionScript`)