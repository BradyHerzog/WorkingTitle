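; BP_Arrow is an arrow projectile actor that flies along an arc and sticks into what it hits.
; Each Tick it sets its pitch from its velocity, keeping roll and yaw, so it follows the trajectory.
; When component E begins overlapping another actor, it stops projectile movement, prints the component name and attaches at the hit bone, keeping world transform.
; It destroys itself after a short delay.
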(event `self.ReceiveTick`
  (params (DeltaSeconds :type "Float (single-precision)"))
  (bind (_returnvalue_roll _returnvalue_pitch _returnvalue_yaw) (`KismetMathLibrary.BreakRotator` (`self.K2_GetActorRotation`)))
  (bind (_returnvalue_roll_2 _returnvalue_pitch_2) (`KismetMathLibrary.BreakRotator` (`KismetMathLibrary.MakeRotFromX` (`self.GetVelocity`))))
  ;[1 1 1] Rotates Arrow to Face Arc
  (`self.K2_SetActorRotation` (`KismetMathLibrary.MakeRotator` _returnvalue_roll _returnvalue_pitch_2 _returnvalue_yaw)))

(event `self.e.OnComponentBeginOverlap`
  (params (OverlappedComponent :type "PrimitiveComponent Object Reference") (OtherActor :type "Actor Object Reference") (OtherComp :type "PrimitiveComponent Object Reference") (OtherBodyIndex :type Integer) (bFromSweep :type Boolean) (SweepResult :type "HitResult Structure (by ref)"))
  (if (!= OtherActor self)
    (`MovementComponent.StopMovementImmediately` (`self.ProjectileMovement`))
    (`KismetSystemLibrary.PrintString` (`KismetSystemLibrary.GetDisplayName` OverlappedComponent))
    (`self.K2_AttachToComponent` OverlappedComponent SweepResult_HitBoneName "KeepWorld" "KeepWorld" "KeepWorld")
    (`KismetSystemLibrary.Delay` 5.0)
    (`self.K2_DestroyActor`)))

(fn `UserConstructionScript`)