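; BP_Draggable_Barrel is a barrel Blueprint, by its name a variant of BP_Draggable, with no finished behavior of its own.
; BeginPlay calls the parent, looks up a BP_Draggable and a BP_Draggable_Barrel in the level, then casts the latter's class to BP_Draggable without using the result.
; Overlap and Tick are disabled, two stray casts never run, and the construction script only calls the parent.
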(event `self.ReceiveBeginPlay`
  (`parent.ReceiveBeginPlay`)
  (`GameplayStatics.GetActorOfClass` "/Game/WorkingTitle/Core/Both/BP_Draggable.BP_Draggable_C")
  (bind _returnvalue (`GameplayStatics.GetActorOfClass` "BP_Draggable_Barrel_C"))
  (castclass `/Game/WorkingTitle/Core/Both/BP_Draggable` (`GameplayStatics.GetObjectClass` _returnvalue)))

(fn `UserConstructionScript`
  (`parent.UserConstructionScript`))