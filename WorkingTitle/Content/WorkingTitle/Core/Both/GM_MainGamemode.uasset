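; Main game mode for an asymmetric session: the first player possesses the top-down camera, and later players get a join pawn to pick a first-person class.
; PlayerSelect checks that the class slot is free in the PlayerClasses map, then spawns and possesses Cleric, Sharpshooter or a base character at a hardcoded location.
; It records the controller against that class and pushes the updated map to every join pawn's buttons.
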(event `self.HandleStartingNewPlayer`
  (params (NewPlayer :type "PlayerController Object Reference"))
  ;[0 0 0] New PlayerJoin
  (bind _returnvalue (`self.GetNumPlayers`))
  (if (== _returnvalue 1)
    (bind _returnvalue_2 (`GameplayStatics.GetActorOfClass` "/Game/WorkingTitle/Core/Topdown/BP_TopDownCamera.BP_TopDownCamera_C"))
    (`Controller.Possess` NewPlayer _returnvalue_2)
    (else
      (bind _returnvalue_3 (`|SpawnActorFromClass` "/Game/WorkingTitle/Core/FirstPerson/Characters/BP_SessionJoinPawn.BP_SessionJoinPawn_C" (`KismetMathLibrary.MakeTransform` (95136.0 50452.0 963.0)) "AdjustIfPossibleButAlwaysSpawn" "OverrideRootScale" NewPlayer null))
      (`Controller.Possess` NewPlayer _returnvalue_3)
      (`/Game/WorkingTitle/Core/FirstPerson/Characters/BP_SessionJoinPawn.UpdateButtonsServer` _returnvalue_3 (`self.PlayerClasses`)))))

(event `PlayerSelect`
  (params (PlayerController :type "PlayerController Object Reference") (DesiredClass :type "/Game/WorkingTitle/Core/FirstPerson/EPLayerClass Enum" :default "NewEnumerator0"))
  (bind _playerclasses (`self.PlayerClasses`))
  (bind _playerclasses_2 (`self.PlayerClasses`))
  (bind _playerclasses_3 (`self.PlayerClasses`))
  (bind _playerclasses_4 (`self.PlayerClasses`))
  (bind (_value _returnvalue) (`BlueprintMapLibrary.Map_Find` (`self.PlayerClasses`) DesiredClass))
  ;[0 0 0] Spawn Player Class
  (if (and (== _value null) _returnvalue)
    (switch `/Game/WorkingTitle/Core/FirstPerson/EPLayerClass` DesiredClass
      (:`NewEnumerator0`
        (bind _returnvalue_2 (`|SpawnActorFromClass` "/Game/WorkingTitle/Core/FirstPerson/Characters/BP_FPChar_Cleric.BP_FPChar_Cleric_C" (`KismetMathLibrary.MakeTransform` (95136.0 50452.0 963.0)) "AdjustIfPossibleButAlwaysSpawn" "OverrideRootScale" PlayerController 100.0 15.0 7.5 null))
        (`Controller.Possess` PlayerController _returnvalue_2)
        (`BlueprintMapLibrary.Map_Remove` _playerclasses_3 "NewEnumerator0")
        (`BlueprintMapLibrary.Map_Add` _playerclasses_3 "NewEnumerator0" PlayerController))
      (:`NewEnumerator1`
        (bind _returnvalue_3 (`|SpawnActorFromClass` "/Game/WorkingTitle/Core/FirstPerson/Characters/BP_FPChar_Sharpshooter.BP_FPChar_Sharpshooter_C" (`KismetMathLibrary.MakeTransform` (95136.0 50452.0 963.0)) "AdjustIfPossibleButAlwaysSpawn" "OverrideRootScale" PlayerController 6 1000.0 250.0 10.0 null))
        (`Controller.Possess` PlayerController _returnvalue_3)
        (`BlueprintMapLibrary.Map_Remove` _playerclasses_4 "NewEnumerator1")
        (`BlueprintMapLibrary.Map_Add` _playerclasses_4 "NewEnumerator1" PlayerController))
      (:`NewEnumerator2`
        (bind _returnvalue_4 (`|SpawnActorFromClass` "/Game/WorkingTitle/Core/FirstPerson/Characters/BP_FPChar_Base.BP_FPChar_Base_C" (`KismetMathLibrary.MakeTransform` (95136.0 50452.0 963.0)) "AdjustIfPossibleButAlwaysSpawn" "OverrideRootScale" PlayerController null))
        (`Controller.Possess` PlayerController _returnvalue_4)
        (`BlueprintMapLibrary.Map_Remove` _playerclasses_2 "NewEnumerator2")
        (`BlueprintMapLibrary.Map_Add` _playerclasses_2 "NewEnumerator2" PlayerController))
      (:`NewEnumerator3`
        (bind _returnvalue_5 (`|SpawnActorFromClass` "/Game/WorkingTitle/Core/FirstPerson/Characters/BP_FPChar_Base.BP_FPChar_Base_C" (`KismetMathLibrary.MakeTransform` (95136.0 50452.0 963.0)) "AdjustIfPossibleButAlwaysSpawn" "OverrideRootScale" PlayerController null))
        (`Controller.Possess` PlayerController _returnvalue_5)
        (`BlueprintMapLibrary.Map_Remove` _playerclasses "NewEnumerator3")
        (`BlueprintMapLibrary.Map_Add` _playerclasses "NewEnumerator3" PlayerController)))
    (bind _outactors (`GameplayStatics.GetAllActorsOfClass` "/Game/WorkingTitle/Core/FirstPerson/Characters/BP_SessionJoinPawn.BP_SessionJoinPawn_C"))
    (for _array_element _outactors
      (`/Game/WorkingTitle/Core/FirstPerson/Characters/BP_SessionJoinPawn.UpdateButtonsServer` _array_element (`self.PlayerClasses`)))))

(fn `UserConstructionScript`)